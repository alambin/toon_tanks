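; Toon Tanks game mode Blueprint that puts up the UI widgets for the match.
; BeginPlay creates the HUD and adds it to the viewport.
; The StartGameBPEvent and GameOverBPEvent events show the start and end game widgets, with the end widget's text set to a win or loss message from IsWinGame.
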(event `self.ReceiveBeginPlay`
  (bind _returnvalue (`|CreateWidget` "/Game/Blueprints/UI/WBP_HUD.WBP_HUD_C"))
  (`UserWidget.AddToViewport` _returnvalue 0))

(event `self.StartGameBPEvent`
  (bind _returnvalue (`|CreateWidget` "/Game/Blueprints/UI/WBP_StartGameWidget.WBP_StartGameWidget_C"))
  (`UserWidget.AddToViewport` _returnvalue 0))

(event `self.GameOverBPEvent`
  (params (IsWinGame :type Boolean))
  (bind _returnvalue (`|CreateWidget` "/Game/Blueprints/UI/WBP_EndGameWidget.WBP_EndGameWidget_C"))
  (`UserWidget.AddToViewport` _returnvalue 0)
  (`TextBlock.SetText` (`/Game/Blueprints/UI/WBP_EndGameWidget.DisplayText` _returnvalue) (select `bool` IsWinGame :`false` "You lost!" :`true` "You won!" :!type "Text")))

(fn `UserConstructionScript`)