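; Base destructible actor that applies an explosion force at a hit location through a physics field.
; ApplyExplosionForceBPEvent spawns an FS_MasterField there, feeds ExplosionForce into its radial and directional magnitudes with the shot direction as vector, then calls CETrigger.
; Unconnected AddRadialForce and AddForceAtLocation nodes remain as alternative approaches that never run.
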(event `self.ApplyExplosionForceBPEvent`
  (params (HitLocation :type "Vector Structure (by ref)") (ShotFromDirection :type "Vector Structure (by ref)"))
  (bind _explosionforce (`self.ExplosionForce`))
  ;[1 1 1] Default method from UE manual (with my extensions to configure field)
  (bind _returnvalue (`|SpawnActorFromClass` "/Engine/EditorResources/FieldNodes/FS_MasterField.FS_MasterField_C" (`KismetMathLibrary.MakeTransform` HitLocation) "Undefined" "OverrideRootScale" null null))
  (set `/Engine/EditorResources/FieldNodes/FS_MasterField.ActivationType` "NewEnumerator4" _returnvalue)
  (set `/Engine/EditorResources/FieldNodes/FS_MasterField.UseDirectionalVector` true _returnvalue)
  (set `/Engine/EditorResources/FieldNodes/FS_MasterField.DirectionalMagnitude` (* _explosionforce 1.0) _returnvalue)
  (set `/Engine/EditorResources/FieldNodes/FS_MasterField.DIrectionalVelocityVector` ShotFromDirection _returnvalue)
  (set `/Engine/EditorResources/FieldNodes/FS_MasterField.Radial Magnitude` _explosionforce _returnvalue)
  (`/Engine/EditorResources/FieldNodes/FS_MasterField.CE_Trigger` _returnvalue))

(fn `UserConstructionScript`)